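; BP_ShooterPlayer is the player character Blueprint, handling basic movement, look and jump input.
; Forward and strafe axes feed AddMovementInput along directions derived from control yaw only, so camera pitch does not affect movement direction.
; Look axes pass straight to controller pitch and yaw, and the Jump press calls the Character's Jump.
; The construction script is empty and no shooting logic is present.
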(fn `UserConstructionScript`)